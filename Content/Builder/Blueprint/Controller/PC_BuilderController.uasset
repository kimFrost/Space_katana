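; Player controller for a builder mode that pans the controlled pawn along fixed world X and Y axes from the Forward and Right inputs.
; Right mouse button toggles a held flag and the zoom actions set a direction value, but neither drives the camera here.
; Pitch and yaw input, the pitch clamp and the zoom offset math are left disconnected, so only movement has a visible effect.
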(event Input|ActionEvents|InputActionZoomIn
  ;[1 1 1] Zoom
  (:Pressed
    (Variables|Default|SetZoomDirection -1)))

(event Input|ActionEvents|InputActionZoomOut
  ;[1 1 1] Zoom
  (:Pressed
    (Variables|Default|SetZoomDirection 1)))

(event Input|AxisEvents|InputAxisLookUp
  (params (AxisValue :type Float%20%28single-precision%29))
  ;[1 1 1] Turn / Look
)

(event Input|AxisEvents|InputAxisTurn
  (params (AxisValue :type Float%20%28single-precision%29))
  ;[1 1 1] Turn / Look
  (if (Variables|Default|GetRightMouseButtonDown)
    _))

(event Input|AxisEvents|InputAxisRight
  (params (AxisValue :type Float%20%28single-precision%29))
  ;[1 1 1] Movement x/y
  (Pawn|Input|AddMovementInput (Pawn|GetControlledPawn) (Math|Vector|MakeVector 0.0 1.0 0.0) AxisValue false))

(event Input|AxisEvents|InputAxisForward
  (params (AxisValue :type Float%20%28single-precision%29))
  ;[1 1 1] Movement x/y
  (Pawn|Input|AddMovementInput (Pawn|GetControlledPawn) (Math|Vector|MakeVector 1.0 0.0 0.0) AxisValue false))

(event Input|MouseEvents|RightMouseButton
  ;[1 1 1] Turn / Look
  (:Pressed
    (Variables|Default|SetRightMouseButtonDown true))
  (:Released
    (Variables|Default|SetRightMouseButtonDown false)))

(fn ConstructionScript)