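; Ship builder actor that spawns a grid of BP_Builder_GridSlot actors on BeginPlay, each given a reference back to the ship.
; UpdateGridSlotsAdjacent tints a slot's four orthogonal neighbours and creates connections to them, or marks existing ones connected.
; Tick draws those connections as debug lines colored by state.
; UpdateGridSlotsInLine recolors slots by row and column; UpdateConnectionsStates is empty and the builder widget creation is unwired.
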(event EventTick
  (params (DeltaSeconds :type Float%20%28single-precision%29))
  ;[1 1 1] Debug Lines for GridSlot Connections
  (bind _array_element (Utilities|Array|ForEachLoopwithBreak (Variables|Default|GetConnectionsList))
    (:LoopBody
      (if (.Connected (Utilities|Struct|BreakST_Connection _array_element))
        (Variables|Temp|Set%25_DebugConnectionColor "(R=0.078057,G=1.000000,B=0.009021,A=1.000000)")
        (else
          (Variables|Temp|Set%25_DebugConnectionColor "(R=0.795000,G=0.023481,B=0.046260,A=1.000000)")))
      (Rendering|Debug|DrawDebugLine (+ (Transformation|GetActorLocation (.Ref1 (Utilities|Struct|BreakST_Connection _array_element))) "0, 0,50.000000") (+ (Transformation|GetActorLocation (.Ref2 (Utilities|Struct|BreakST_Connection _array_element))) "0, 0,50.000000") (Variables|Temp|Get%25_DebugConnectionColor) 0.1 5.0))))

(event EventBeginPlay
  (bind _gridslotsize (Variables|Default|GetGridSlotSize))
  (Utilities|FlowControl|Sequence
    (:then_2
      (for _index (range 0 (Variables|Default|GetGridRowCount))
        (for _index_2 (range 0 (Variables|Default|GetGridColumCount))
          (bind _returnvalue (Game|SpawnActorfromClass "/Game/Builder/Blueprint/Actor/BP_Builder_GridSlot.BP_Builder_GridSlot_C" (Math|Transform|MakeTransform (Math|Vector|MakeVector (* _index _gridslotsize) (* _index_2 _gridslotsize) 0.0)) true _index _index_2 0))
          (bind _returnvalue_2 (Utilities|Array|Add (Variables|Default|GetGridSlots) _returnvalue))
          (Variables|/Game/Builder/Blueprint/Actor/BP_Builder_GridSlot.BP_Builder_GridSlot_C|SetIndex _returnvalue _returnvalue_2)
          (Variables|/Game/Builder/Blueprint/Actor/BP_Builder_GridSlot.BP_Builder_GridSlot_C|SetShipRef _returnvalue self))))))

(fn ConstructionScript)

(fn UpdateGridSlotsAdjacent
  (params (Column :type Integer) (Row :type Integer) (GridSlot :type BP%20Builder%20Grid%20Slot%20Object%20Reference))
  (bind _connectionslist (Variables|Default|GetConnectionsList))
  (bind _gridcolumcount (Variables|Default|GetGridColumCount))
  (Variables|Temp|Set%25_Column Column)
  (Variables|Temp|Set%25_Row Row)
  (Utilities|Array|Clear (Variables|Temp|Get%25_Connections))
  (Variables|Temp|Set%25_GridSlot GridSlot)
  (Utilities|FlowControl|Sequence
    (:then_0
      ;[1 1 1] Make CoordsList (Top, Right, Bottom, Left)
      (Variables|Temp|Set%25_CoordsList (Utilities|Array|MakeArray (Utilities|Struct|MakeST_Cords (Variables|Temp|Get%25_Column) (+ (Variables|Temp|Get%25_Row) 1)) (Utilities|Struct|MakeST_Cords (+ (Variables|Temp|Get%25_Column) 1) (Variables|Temp|Get%25_Row)) (Utilities|Struct|MakeST_Cords (Variables|Temp|Get%25_Column) (- (Variables|Temp|Get%25_Row) 1)) (Utilities|Struct|MakeST_Cords (- (Variables|Temp|Get%25_Column) 1) (Variables|Temp|Get%25_Row)))))
    (:then_1
      (for _array_element (Variables|Temp|Get%25_CoordsList)
        (Variables|Temp|Set%25_X (.X (Utilities|Struct|BreakST_Cords _array_element)))
        (Variables|Temp|Set%25_Y (.Y (Utilities|Struct|BreakST_Cords _array_element)))
        (if (Math|Boolean|ANDBoolean (<= (Variables|Temp|Get%25_X) _gridcolumcount) (>= (Variables|Temp|Get%25_Y) 0) (>= (Variables|Temp|Get%25_X) 0) (< (Variables|Temp|Get%25_Y) (/ (Utilities|Array|Length (Variables|Default|GetGridSlots)) _gridcolumcount)))
          (Variables|Temp|Set%25_AdjacentGridSlot (Utilities|Array|Get(acopy) (Variables|Default|GetGridSlots) (Utilities|GetGridIndex _gridcolumcount (Variables|Temp|Get%25_X) (Variables|Temp|Get%25_Y))))
          (Rendering|Material|SetVectorParameterValue (Variables|/Game/Builder/Blueprint/Actor/BP_Builder_GridSlot.BP_Builder_GridSlot_C|GetMaterial (Utilities|Array|Get(acopy) (Variables|Default|GetGridSlots) (Utilities|GetGridIndex _gridcolumcount (Variables|Temp|Get%25_X) (Variables|Temp|Get%25_Y)))) "Color" "(R=0.122868,G=1.000000,B=0.033356,A=1.000000)" :!class /Script/Engine.MaterialInstanceDynamic)
          ;[1 1 1] Create/Update Connection between adjacent GridSlots
          (Variables|Temp|Set%25_Found false)
          (Variables|Temp|Set%25_Break false)
          (bind (_array_element_2 _array_index) (Utilities|Array|ForEachLoopwithBreak (Variables|Default|GetConnectionsList) :!label _label)
            (:LoopBody
              (if (Variables|Temp|Get%25_Break)
                (goto _label Break)
                (else
                  (Variables|Temp|Set%25_Index _array_index)
                  (if (or (and (Utilities|ActorIsActor (.Ref1 (Utilities|Struct|BreakST_Connection _array_element_2)) (Variables|Temp|Get%25_GridSlot)) (Utilities|ActorIsActor (.Ref2 (Utilities|Struct|BreakST_Connection _array_element_2)) (Variables|Temp|Get%25_AdjacentGridSlot))) (and (Utilities|ActorIsActor (.Ref1 (Utilities|Struct|BreakST_Connection _array_element_2)) (Variables|Temp|Get%25_AdjacentGridSlot)) (Utilities|ActorIsActor (.Ref2 (Utilities|Struct|BreakST_Connection _array_element_2)) (Variables|Temp|Get%25_GridSlot))))
                    (Variables|Temp|Set%25_Found true)
                    ;[1 1 1] Update Connection
                    (Development|PrintString "Update Connection")
                    (Utilities|Array|SetArrayElem _connectionslist (Variables|Temp|Get%25_Index) (Utilities|Struct|MakeST_Connection "None" (.Ref1 (Utilities|Struct|BreakST_Connection (Utilities|Array|Get(acopy) _connectionslist (Variables|Temp|Get%25_Index)))) (.Ref2 (Utilities|Struct|BreakST_Connection (Utilities|Array|Get(acopy) _connectionslist (Variables|Temp|Get%25_Index)))) true))))))
            (:Completed
              (if (not (Variables|Temp|Get%25_Found))
                ;[1 1 1] Create  Connection
                (Development|PrintString "Create Connection")
                (Utilities|Array|Add (Variables|Default|GetConnectionsList) (Utilities|Struct|MakeST_Connection "None" (Variables|Temp|Get%25_GridSlot) (Variables|Temp|Get%25_AdjacentGridSlot) false))))))))))

(fn UpdateGridSlotsinLine
  (params (Column :type Integer) (Row :type Integer))
  (Variables|Temp|Set%25_Column Column)
  (Variables|Temp|Set%25_Row Row)
  (bind _array_element (Utilities|Array|ForEachLoopwithBreak (Variables|Default|GetGridSlots))
    (:LoopBody
      (if (== (Variables|/Game/Builder/Blueprint/Actor/BP_Builder_GridSlot.BP_Builder_GridSlot_C|GetRow _array_element) (Variables|Temp|Get%25_Row))
        (if (== (Variables|/Game/Builder/Blueprint/Actor/BP_Builder_GridSlot.BP_Builder_GridSlot_C|GetColumn _array_element) (Variables|Temp|Get%25_Column))
          (Rendering|Material|SetVectorParameterValue (Variables|/Game/Builder/Blueprint/Actor/BP_Builder_GridSlot.BP_Builder_GridSlot_C|GetMaterial _array_element) "Color" "(R=1.000000,G=0.018015,B=0.000000,A=1.000000)" :!class /Script/Engine.MaterialInstanceDynamic :!label _label)
          (else
            (Rendering|Material|SetVectorParameterValue (Variables|/Game/Builder/Blueprint/Actor/BP_Builder_GridSlot.BP_Builder_GridSlot_C|GetMaterial _array_element) "Color" "(R=0.000000,G=0.323203,B=0.760000,A=1.000000)" :!class /Script/Engine.MaterialInstanceDynamic :!label _label_2)))
        (elif (== (Variables|/Game/Builder/Blueprint/Actor/BP_Builder_GridSlot.BP_Builder_GridSlot_C|GetColumn _array_element) (Variables|Temp|Get%25_Column))
          (goto _label_2)
          (else
            (goto _label)))))))

(fn UpdateConnectionsStates)