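; BP_Builder_GridSlot is a grid slot actor for the builder that highlights when the cursor hovers over it.
; Construction creates a dynamic instance of M_BuilderSlot on its static mesh with a red default Color.
; Cursor enter tints it pale lavender, prints its name and calls GridSlotMouseOver with itself; cursor exit restores red.
; Click and release handlers are empty, and several leftover material and debug-draw nodes never run.
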(event EventActorBeginCursorOver
  (Development|PrintString (Utilities|GetDisplayName self))
  (Rendering|Material|SetVectorParameterValue (Variables|Default|GetMaterial) "Color" "(R=0.847932,G=0.760000,B=1.000000,A=1.000000)" :!class /Script/Engine.MaterialInstanceDynamic)
  (Default|CallGridSlotMouseOver self))

(event EventActorEndCursorOver
  (Rendering|Material|SetVectorParameterValue (Variables|Default|GetMaterial) "Color" "(R=1.000000,G=0.065432,B=0.000000,A=1.000000)" :!class /Script/Engine.MaterialInstanceDynamic))

(event EventActorOnClicked)

(event EventActorOnReleased)

(fn ConstructionScript
  (bind _returnvalue (Rendering|Material|CreateDynamicMaterialInstance "/Game/Builder/Material/M_BuilderSlot.M_BuilderSlot" :!class /Script/Engine.KismetMaterialLibrary))
  (Variables|Default|SetMaterial _returnvalue)
  (Rendering|Material|SetMaterial (Variables|Default|GetStaticMesh1) 0 (Variables|Default|GetMaterial))
  (Rendering|Material|SetVectorParameterValue (Variables|Default|GetMaterial) "Color" "(R=1.000000,G=0.065432,B=0.000000,A=1.000000)" :!class /Script/Engine.MaterialInstanceDynamic))