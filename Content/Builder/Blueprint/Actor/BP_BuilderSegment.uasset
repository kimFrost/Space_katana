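; BP_BuilderSegment is a clickable builder segment actor that stores connections to top, right, bottom and left segments through SetConnections.
; Its construction script adds the segment mesh and casts each connection, but only a valid top connection adds a small pyramid mesh.
; Clicks only print debug text.
; The code creating four surrounding Add meshes and binding their click handlers is disconnected and never runs.
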(event Custom|OnClicked_Event_Component3
  (params (TouchedComponent :type Primitive%20Component%20Object%20Reference))
  (Development|PrintString "Add Component Clicked - Bottom"))

(event Custom|OnClicked_Event_Component4
  (params (TouchedComponent :type Primitive%20Component%20Object%20Reference))
  (Development|PrintString "Add Component Clicked - left")
  (bind _returnvalue (Transformation|GetRelativeTransform TouchedComponent))
  (Development|PrintString (Utilities|String|ToString(Vector) (.Location (Math|Transform|BreakTransform _returnvalue)))))

(event Custom|OnClicked_Event_Component1
  (params (TouchedComponent :type Primitive%20Component%20Object%20Reference))
  (Development|PrintString "Add Component Clicked - Top"))

(event Custom|OnClicked_Event_Component2
  (params (TouchedComponent :type Primitive%20Component%20Object%20Reference))
  (Development|PrintString "Add Component Clicked - Right"))

(event EventBeginPlay)

(event EventActorOnReleased)

(event EventActorOnClicked
  (Development|PrintString (Utilities|String|Append "Clicked On Segment: " (Utilities|GetDisplayName self))))

(fn ConstructionScript
  (Utilities|FlowControl|Sequence
    (:then_0
      (bind _returnvalue (AddComponent|AddStaticMeshComponent true (Math|Transform|MakeTransform "0, 0, 0")))
      (Components|StaticMesh|SetStaticMesh _returnvalue "/Game/Builder/Mesh/Segment/Segment.Segment")
      (Class|SceneComponent|Attachto _returnvalue (VehicleSound|GetRootComponent) "None" "KeepRelativeOffset" true))
    (:then_1
      (Utilities|FlowControl|Sequence
        (:then_0
          (Utilities|Casting|CastToBP_BuilderSegment (.Ref1 (Utilities|Struct|BreakST_Connection (Variables|Default|GetConnectionTop))))
          (bind _returnvalue_2 (AddComponent|AddStaticMeshComponent false (Math|Transform|MakeTransform "25.000000,0.000000,52.000000" "0, 0, 0" "0.100000,0.100000,0.100000")))
          (Components|StaticMesh|SetStaticMesh _returnvalue_2 "/Game/Shapes/Shape_QuadPyramid.Shape_QuadPyramid"))
        (:then_1
          (Utilities|Casting|CastToBP_BuilderSegment (.Ref1 (Utilities|Struct|BreakST_Connection (Variables|Default|GetConnectionRight)))))
        (:then_2
          (Utilities|Casting|CastToBP_BuilderSegment (.Ref1 (Utilities|Struct|BreakST_Connection (Variables|Default|GetConnectionBottom)))))
        (:then_3
          (Utilities|Casting|CastToBP_BuilderSegment (.Ref1 (Utilities|Struct|BreakST_Connection (Variables|Default|GetConnectionLeft)))))))))

(fn SetConnections
  (params (Top :type ST%20Connection%20Structure) (Right :type ST%20Connection%20Structure) (Bottom :type ST%20Connection%20Structure) (Left :type ST%20Connection%20Structure))
  (Variables|Default|SetConnectionTop Top)
  (Variables|Default|SetConnectionRight Right)
  (Variables|Default|SetConnectionBottom Bottom)
  (Variables|Default|SetConnectionLeft Left))