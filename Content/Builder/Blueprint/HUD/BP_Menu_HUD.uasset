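; Main menu HUD that draws New Game, Load Builder and Exit Game buttons on the canvas, plus debug strings at top right.
; DrawButton pairs centered text and a texture with a hitbox, whose release events open the game or builder level, or quit.
; Level opens set a Loading flag and use a zero Delay before loading, for the bottom-right "Loading" text.
; A Log helper files messages by category.
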(event EventDrawHUD
  (params (SizeX :type Integer) (SizeY :type Integer))
  (bind _returnvalue (Math|Conversions|ToFloat(Integer) SizeX))
  (bind _returnvalue_2 (Math|Conversions|ToFloat(Integer) SizeY))
  (bind (_outwidth _outheight) (Class|HUD|GetTextSize "Loading" "/Engine/EngineFonts/RobotoDistanceField.RobotoDistanceField" 1.0))
  (bind (_outwidth_2 _outheight_2) (Class|HUD|GetTextSize "" "/Engine/EditorResources/SmallFont.SmallFont" 1.0))
  (bind _returnvalue_3 (Math|Vector2D|MakeVector2D _returnvalue _returnvalue_2))
  (Variables|Default|SetGameStateObject (Game|GetGameState))
  ;[1 1 1] Set Screen Dimensions
  (Variables|Default|SetScreenDimensions _returnvalue_3)
  (Variables|Default|SetScreenCenterDimensions (/ _returnvalue_3 2.0))
  ;[1 1 1] Draw Debug Strings
  (for (_ _array_index) 0
    (HUD|DrawText :ScreenX (- (- (.X (Math|Vector2D|BreakVector2D (Variables|Default|GetScreenDimensions))) _outwidth_2) 5.0) :ScreenY (+ (* _array_index _outheight_2) 5.0) :Font "/Engine/EditorResources/SmallFont.SmallFont"))
  ;[1 1 1] Draw Menu
  (if (Variables|Default|GetShowMenu)
    (CallFunction|DrawButton (- (Variables|Default|GetScreenCenterDimensions) (Math|Vector2D|MakeVector2D 0.0 0.0)) "New Game" "NewGame" (select false 0 0))
    (CallFunction|DrawButton (+ (Variables|Default|GetScreenCenterDimensions) (Math|Vector2D|MakeVector2D 0.0 64.0)) "Load Builder" "LoadBuilder" (select false 0 0))
    (CallFunction|DrawButton (+ (Variables|Default|GetScreenCenterDimensions) (Math|Vector2D|MakeVector2D 0.0 128.0)) "Exit Game" "ExitGame" (select false 0 0))
    ;[1 1 1] Draw Loading Screen
    (Utilities|Casting|CastTo (Game|GetGameInstance))
    (if (Variables|Default|GetLoading)
      (HUD|DrawText "Loading" "(R=0.420133,G=0.068875,B=0.725000,A=1.000000)" (- (.X (Math|Vector2D|BreakVector2D (- (Variables|Default|GetScreenDimensions) (Math|Vector2D|MakeVector2D 2e+01 2e+01)))) _outwidth) (- (.Y (Math|Vector2D|BreakVector2D (- (Variables|Default|GetScreenDimensions) (Math|Vector2D|MakeVector2D 2e+01 2e+01)))) _outheight) 0 1.0 false))))

(event EventHitBoxClick
  (params (BoxName :type Name :default "None"))
  ;[1 1 1] Hit box events
  (switch name BoxName))

(event EventHitBoxRelease
  (params (BoxName :type Name :default "None"))
  (bind _returnvalue (Game|GetGameInstance))
  ;[1 1 1] Hit box events
  (switch name BoxName
    (:NewGame
      (Utilities|Casting|CastTo _returnvalue)
      (Variables|Default|SetLoading true)
      (Utilities|FlowControl|Delay 0.0)
      (Game|OpenLevel(byName) "Minimal_Default" false))
    (:ExitGame
      (Game|QuitGame))
    (:LoadBuilder
      (Utilities|Casting|CastTo _returnvalue)
      (Variables|Default|SetLoading true)
      (Utilities|FlowControl|Delay 0.0)
      (Game|OpenLevel(byName) "Bombartment_builder" false))))

(fn ConstructionScript)

(fn DrawButton
  (params (Screen%20location :type Vector%202D%20Structure) (Text :type String) (Hitbox%20Name :type Name) (Texture :type Texture%202D%20Object%20Reference))
  (bind _returnvalue (Math|Vector2D|MakeVector2D 128.0 64.0))
  (bind (_outwidth _outheight) (Class|HUD|GetTextSize Text "/Engine/EngineFonts/RobotoDistanceField.RobotoDistanceField" 1.5))
  (bind _returnvalue_2 (Math|Vector2D|MakeVector2D _outwidth _outheight))
  (bind _returnvalue_3 (- Screen%20location _returnvalue))
  (bind (_x _y) (Math|Vector2D|BreakVector2D _returnvalue_3))
  (bind _returnvalue_4 (/ _returnvalue_2 2.0))
  (bind _returnvalue_5 (- Screen%20location _returnvalue_4))
  (bind (_x_2 _y_2) (Math|Vector2D|BreakVector2D _returnvalue_5))
  (Class|HUD|DrawTextureSimple Texture _x _y 1.0 false)
  (HUD|DrawText Text "(R=1.000000,G=1.000000,B=1.000000,A=1.000000)" _x_2 _y_2 "/Engine/EngineFonts/RobotoDistanceField.RobotoDistanceField" 1.5 false)
  (Class|HUD|AddHitBox _returnvalue_3 (Math|Vector2D|MakeVector2D 256.0 128.0) Hitbox%20Name false))

(fn Log
  (params (msg :type String) (Category :type Name) (print :type Boolean))
  (bind _returnvalue (Utilities|Name|Equal(Name) Category "None"))
  (LocalVariables|SetFound false)
  (LocalVariables|SetCategoryName Category)
  (bind (_array_element _array_index) (Utilities|Array|ForEachLoopwithBreak 0 :!label _label)
    (:LoopBody
      (LocalVariables|SetCategotyItem _array_element)
      (if _returnvalue
        (LocalVariables|SetFound _returnvalue)
        (LocalVariables|SetFoundAtIndex _array_index)
        (goto _label Break)))
    (:Completed
      (if (LocalVariables|GetFound)
        _
        (else
          (bind _returnvalue_2 (Utilities|Array|Add 0 "0"))
          (LocalVariables|SetFoundAtIndex _returnvalue_2)))
      (if print
        (Utilities|Array|Add 0 "0")))))