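; HUD Blueprint for a builder interface: a selectable tile grid, a tool tab bar with module or segment buttons, and a debug readout.
; Canvas functions draw each element and register named hit boxes, whose release events update tile and tool structs.
; DebugThis keeps a name/value list for the overlay.
; The drawing sequence is disconnected from DrawHUD, and tool selection is unfinished, with UpdateValues always picking the last tool.
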(event EventDrawHUD
  (params (SizeX :type Integer) (SizeY :type Integer)))

(event EventBeginPlay)

(event EventHitBoxClick
  (params (BoxName :type Name :default "None")))

(event EventHitBoxBeginCursorOver
  (params (BoxName :type Name :default "None"))
  (Variables|Temp|SetHitBoxOverName BoxName)
  (Debug|DebugThis "HitBoxOverName" (Utilities|String|ToString(Name) BoxName)))

(event EventHitBoxEndCursorOver
  (params (BoxName :type Name :default "None"))
  (Variables|Temp|SetHitBoxOverEndName BoxName)
  (Debug|DebugThis "HitBoxOverEndName" (Utilities|String|ToString(Name) BoxName)))

(event EventHitBoxRelease
  (params (BoxName :type Name :default "None"))
  (bind _toolsliststruct (Variables|Tools|GetToolsListStruct))
  (bind _toollist (Utilities|Struct|BreakST_Tools _toolsliststruct))
  (Variables|Temp|SetHitBoxClickName BoxName)
  (Utilities|FlowControl|Sequence
    (:then_0
      ;[1 1 1] Grid
      (bind (_array_element _array_index) (Utilities|Array|ForEachLoopwithBreak (Variables|Default|GetTilesList))
        (:LoopBody
          (if (Math|Boolean|ORBoolean (Utilities|Name|Equal(Name) (Variables|Temp|GetHitBoxClickName) (.ID (Utilities|Struct|BreakST_GridTile _array_element))) false false)
            (Utilities|Array|SetArrayElem (Variables|Default|GetTilesList) _array_index (Utilities|Struct|MakeST_GridTile (.IndexX (Utilities|Struct|BreakST_GridTile _array_element)) (.IndexY (Utilities|Struct|BreakST_GridTile _array_element)) (.ID (Utilities|Struct|BreakST_GridTile _array_element)) (.ModuleComponentID (Utilities|Struct|BreakST_GridTile _array_element)) (Utilities|Struct|MakeST_GridStates (Utilities|Name|Equal(Name) (Variables|Temp|GetHitBoxClickName) (.ID (Utilities|Struct|BreakST_GridTile _array_element))) true false false)))))))
    (:then_1
      ;[1 1 1] Tools
      (for (_array_element_2 _array_index_2) (.ToolList (Utilities|Struct|BreakST_Tools (Variables|Tools|GetToolsListStruct)))
        (if (Utilities|Name|Equal(Name) (Variables|Temp|GetHitBoxClickName) (.ID (Utilities|Struct|BreakST_Tool _array_element_2)))
          (Utilities|Array|SetArrayElem _toollist _array_index_2 (Utilities|Struct|MakeST_Tool (.ID (Utilities|Struct|BreakST_Tool _array_element_2)) (.Title (Utilities|Struct|BreakST_Tool _array_element_2)) (Utilities|Array|MakeArray "")))
          (for (_array_element_3 _array_index_3) _toollist
            (if (Utilities|Name|NotEqual(Name) (.ID (Utilities|Struct|BreakST_Tool _array_element_3)) (Variables|Temp|GetHitBoxClickName))
              (Utilities|Array|SetArrayElem _toollist _array_index_3 (Utilities|Struct|MakeST_Tool (.ID (Utilities|Struct|BreakST_Tool _array_element_3)) (.Title (Utilities|Struct|BreakST_Tool _array_element_3)) (Utilities|Array|MakeArray ""))))))))))

(fn ConstructionScript)

(fn CreateTileGrid
  ;[1 1 1] Loop From Top line to bottom
  (for _index (range 1 (Variables|Grid|GetGridTilesY))
    (Variables|Temp|SetIndexY _index)
    ;[1 1 1] Loop From left to right
    (for _index_2 (range 1 (Variables|Grid|GetGridTilesX))
      (Variables|Temp|SetIndexX _index_2)
      ;[1 1 1] Create Tile and append to TilesList
      (Utilities|Array|Add (Variables|Default|GetTilesList) (Utilities|Struct|MakeST_GridTile (Variables|Temp|GetIndexX) (Variables|Temp|GetIndexY) (Utilities|String|StringToName (Utilities|String|Append (Utilities|String|ToString(Integer) (Variables|Temp|GetIndexX)) (Utilities|String|ToString(Integer) (Variables|Temp|GetIndexY)))))))))

(fn DrawTileGrid
  (bind _gridsize (Variables|Grid|GetGridSize))
  (bind _gridsize_2 (Variables|Grid|GetGridSize))
  (bind _gridsize_3 (Variables|Grid|GetGridSize))
  (bind _gridsize_4 (Variables|Grid|GetGridSize))
  (LocalVariables|Set%25_DrawPos (- (Variables|Grid|GetGridOffset) (Math|Vector2D|MakeVector2D _gridsize_2 _gridsize_2)))
  (for _array_element (Variables|Default|GetTilesList)
    (LocalVariables|Set%25_tileIndexX (.IndexX (Utilities|Struct|BreakST_GridTile _array_element)))
    (LocalVariables|Set%25_tileIndexY (.IndexY (Utilities|Struct|BreakST_GridTile _array_element)))
    (LocalVariables|Set%25_tilePosX (+ (* (LocalVariables|Get%25_tileIndexX) _gridsize) (.X (Math|Vector2D|BreakVector2D (LocalVariables|Get%25_DrawPos)))))
    (LocalVariables|Set%25_tilePosY (+ (* (LocalVariables|Get%25_tileIndexY) _gridsize) (.Y (Math|Vector2D|BreakVector2D (LocalVariables|Get%25_DrawPos)))))
    (LocalVariables|Set%25_tileID (.ID (Utilities|Struct|BreakST_GridTile _array_element)))
    (LocalVariables|Set%25_tileModuleID (.ModuleComponentID (Utilities|Struct|BreakST_GridTile _array_element)))
    (LocalVariables|Set%25_tileSelected (.Selected (Utilities|Struct|BreakST_GridStates (.States (Utilities|Struct|BreakST_GridTile _array_element)))))
    (LocalVariables|Set%25_TileHover (.Hover (Utilities|Struct|BreakST_GridStates (.States (Utilities|Struct|BreakST_GridTile _array_element)))))
    (HUD|DrawRect (Math|Color|SelectColor "(R=0.880412,G=0.905516,B=0.955000,A=1.000000)" "(R=0.067019,G=0.242791,B=0.325000,A=1.000000)" (LocalVariables|Get%25_tileSelected)) (LocalVariables|Get%25_tilePosX) (LocalVariables|Get%25_tilePosY) _gridsize_4 _gridsize_4)
    (Class|HUD|DrawLine (LocalVariables|Get%25_tilePosX) (LocalVariables|Get%25_tilePosY) (+ (LocalVariables|Get%25_tilePosX) _gridsize_4) (LocalVariables|Get%25_tilePosY) (Math|Color|SelectColor "(R=0.000000,G=0.895000,B=0.175242,A=1.000000)" "(R=0.940000,G=0.241295,B=0.470165,A=1.000000)" (LocalVariables|Get%25_TileHover)))
    (Class|HUD|DrawLine (LocalVariables|Get%25_tilePosX) (LocalVariables|Get%25_tilePosY) (LocalVariables|Get%25_tilePosX) (+ (LocalVariables|Get%25_tilePosY) _gridsize_4) "(R=0.000000,G=0.000000,B=0.000000,A=1.000000)")
    (Class|HUD|AddHitBox (Math|Vector2D|MakeVector2D (LocalVariables|Get%25_tilePosX) (LocalVariables|Get%25_tilePosY)) (Math|Vector2D|MakeVector2D _gridsize_3 _gridsize_3) (LocalVariables|Get%25_tileID) false)))

(fn DrawTools
  (bind _toolsliststruct (Variables|Tools|GetToolsListStruct))
  (bind _toolswindowpos (Variables|Tools|GetToolsWindowPos))
  (bind _toolsbuttonheight (Variables|Tools|GetToolsButtonHeight))
  (bind _toollist (Utilities|Struct|BreakST_Tools _toolsliststruct))
  (bind (_x _y) (Math|Vector2D|BreakVector2D _toolswindowpos))
  (LocalVariables|Set_ToolButtonWidth (/ (Variables|Tools|GetToolsWindowWidth) (Math|Conversions|ToFloat(Integer) (Utilities|Array|Length _toollist))))
  (for (_array_element _array_index) _toollist
    (LocalVariables|Set_ToolIndex _array_index)
    (HUD|DrawRect (Math|Color|SelectColor "(R=0.325000,G=0.010986,B=0.108431,A=1.000000)" "(R=0.038473,G=0.000005,B=0.003303,A=1.000000)" false) (+ _x (* (LocalVariables|Get_ToolIndex) (LocalVariables|Get_ToolButtonWidth))) _y (LocalVariables|Get_ToolButtonWidth) _toolsbuttonheight)
    (HUD|DrawText (.Title (Utilities|Struct|BreakST_Tool _array_element)) "(R=0.676420,G=0.598500,B=0.950000,A=1.000000)" (+ _x (* (LocalVariables|Get_ToolIndex) (LocalVariables|Get_ToolButtonWidth))) _y 0 1.0 false)
    (Class|HUD|AddHitBox (Math|Vector2D|MakeVector2D (+ _x (* (LocalVariables|Get_ToolIndex) (LocalVariables|Get_ToolButtonWidth))) _y) (Math|Vector2D|MakeVector2D (LocalVariables|Get_ToolButtonWidth) _toolsbuttonheight) (.ID (Utilities|Struct|BreakST_Tool _array_element)) false)))

(fn CreateTools
  (for _array_element (.ToolList (Utilities|Struct|BreakST_Tools (Variables|Tools|GetToolsListStruct)))
    _))

(fn DrawDebug
  (bind _debuglist (Variables|Debug|GetDebugList))
  (bind _screendimensions (Variables|Default|GetScreenDimensions))
  (bind _y (Math|Vector2D|BreakVector2D _screendimensions))
  (bind _returnvalue (- _y 2e+02))
  (HUD|DrawRect "(R=0.000000,G=0.000000,B=0.000000,A=0.823000)" 5e+01 _returnvalue 2e+02 (* (Utilities|Array|Length _debuglist) (Variables|Debug|GetDebugTextHeight)))
  (for (_array_element _array_index) _debuglist
    (HUD|DrawText (Utilities|String|BuildString(Name) (Utilities|String|ToString(Name) (.Name (Utilities|Struct|BreakST_Debugitem _array_element))) " : " (Utilities|String|StringToName (.Value (Utilities|Struct|BreakST_Debugitem _array_element))) "") "(R=1.000000,G=1.000000,B=1.000000,A=1.000000)" 6e+01 (+ (* _array_index (Variables|Debug|GetDebugTextHeight)) _returnvalue) 0 1.0 false)))

(fn DebugThis
  (params (Name :type Name) (Value :type String))
  (bind (_array_element _array_index) (Utilities|Array|ForEachLoopwithBreak (Variables|Debug|GetDebugList) :!label _label)
    (:LoopBody
      (if (Utilities|Name|Equal(Name) (.Name (Utilities|Struct|BreakST_Debugitem _array_element)) Name)
        (LocalVariables|SetFoundAny true)
        (Utilities|Array|SetArrayElem (Variables|Debug|GetDebugList) _array_index (Utilities|Struct|MakeST_Debugitem (.Name (Utilities|Struct|BreakST_Debugitem _array_element)) Value))
        (goto _label Break)))
    (:Completed
      (if (not (LocalVariables|GetFoundAny))
        (Utilities|Array|Add (Variables|Debug|GetDebugList) (Utilities|Struct|MakeST_Debugitem Name Value))))))

(fn DrawToolContent
  (bind _toolsbuttonheight (Variables|Tools|GetToolsButtonHeight))
  (bind _toolswindowpos (Variables|Tools|GetToolsWindowPos))
  (bind _toolscontentitemperline (Variables|Tools|GetToolsContentItemPerLine))
  (bind _toolscontentitemperline_2 (Variables|Tools|GetToolsContentItemPerLine))
  (bind _toolsbuttonheight_2 (Variables|Tools|GetToolsButtonHeight))
  (bind _toolscontentmargin (Variables|Tools|GetToolsContentMargin))
  (bind _toolscontentitemspacing (Variables|Tools|GetToolsContentItemSpacing))
  (bind _selectedtool (Variables|Global|GetSelectedTool))
  (bind _toolssegments (Variables|Tools|GetToolsSegments))
  (bind _toolsmodules (Variables|Tools|GetToolsModules))
  (bind _toolswindowpos_2 (Variables|Tools|GetToolsWindowPos))
  (bind (_modulelist _id) (Utilities|Struct|BreakST_Modules _toolsmodules))
  (bind (_segmentlist _id_2) (Utilities|Struct|BreakST_Segments _toolssegments))
  (bind _returnvalue (Math|Vector2D|MakeVector2D 0.0 _toolsbuttonheight))
  (bind (_x _y) (Math|Vector2D|BreakVector2D _toolswindowpos_2))
  (bind _returnvalue_2 (+ _returnvalue _toolswindowpos))
  (bind (_x_2 _y_2) (Math|Vector2D|BreakVector2D _returnvalue_2))
  (Utilities|FlowControl|Sequence
    (:then_0
      (LocalVariables|Set%25_ToolsContentItemWidth (/ (- (- (Variables|Tools|GetToolsWindowWidth) (* 2 (Variables|Tools|GetToolsContentMargin))) (* (- _toolscontentitemperline_2 1) (Variables|Tools|GetToolsContentItemSpacing))) (Math|Conversions|ToFloat(Integer) _toolscontentitemperline_2)))
      (HUD|DrawRect "(R=0.000000,G=0.000000,B=0.000000,A=0.800000)" _x_2 _y_2 (Variables|Tools|GetToolsWindowWidth) 4e+02)
      (if (Utilities|Name|Equal(Name) _selectedtool _id)
        (for (_array_element _array_index) _modulelist
          (LocalVariables|Set%25_i _array_index)
          (LocalVariables|Set%25_ID (.ID (Utilities|Struct|BreakST_Module _array_element)))
          (LocalVariables|Set%25_title (.Title (Utilities|Struct|BreakST_Module _array_element)))
          (Utilities|FlowControl|Sequence
            (:then_0
              (Utilities|FlowControl|Sequence
                (:then_0
                  (LocalVariables|Set%25_ButtonXIndex (Math|Integer|%(Integer) (LocalVariables|Get%25_i) _toolscontentitemperline))
                  (LocalVariables|Set%25_ButtonYIndex (/ (LocalVariables|Get%25_i) _toolscontentitemperline))
                  (LocalVariables|Set%25_ButtonX (+ (* (LocalVariables|Get%25_ButtonXIndex) (LocalVariables|Get%25_ToolsContentItemWidth)) (+ _x _toolscontentmargin (* (LocalVariables|Get%25_ButtonXIndex) _toolscontentitemspacing))))
                  (LocalVariables|Set%25_ButtonY (+ (+ (* (LocalVariables|Get%25_ButtonYIndex) _toolsbuttonheight_2) _toolsbuttonheight_2) (+ _y _toolscontentmargin (* (LocalVariables|Get%25_ButtonYIndex) _toolscontentitemspacing))))
                  (LocalVariables|Set%25_ButtonLeftTopPos (Math|Vector2D|MakeVector2D (+ (* (LocalVariables|Get%25_ButtonXIndex) (LocalVariables|Get%25_ToolsContentItemWidth)) (+ _x _toolscontentmargin (* (LocalVariables|Get%25_ButtonXIndex) _toolscontentitemspacing))) (+ (+ (* (LocalVariables|Get%25_ButtonYIndex) _toolsbuttonheight_2) _toolsbuttonheight_2) (+ _y _toolscontentmargin (* (LocalVariables|Get%25_ButtonYIndex) _toolscontentitemspacing)))))
                  (LocalVariables|Set%25_ButtonRightBottomPos (+ (Math|Vector2D|MakeVector2D (+ (* (LocalVariables|Get%25_ButtonXIndex) (LocalVariables|Get%25_ToolsContentItemWidth)) (+ _x _toolscontentmargin (* (LocalVariables|Get%25_ButtonXIndex) _toolscontentitemspacing))) (+ (+ (* (LocalVariables|Get%25_ButtonYIndex) _toolsbuttonheight_2) _toolsbuttonheight_2) (+ _y _toolscontentmargin (* (LocalVariables|Get%25_ButtonYIndex) _toolscontentitemspacing)))) (Math|Vector2D|MakeVector2D (LocalVariables|Get%25_ToolsContentItemWidth) _toolsbuttonheight_2))))))
            (:then_1
              (HUD|DrawRect "(R=0.208383,G=0.540137,B=0.995000,A=1.000000)" (LocalVariables|Get%25_ButtonX) (LocalVariables|Get%25_ButtonY) (LocalVariables|Get%25_ToolsContentItemWidth) (Variables|Tools|GetToolsButtonHeight))
              (HUD|DrawText (LocalVariables|Get%25_title) "(R=0.335000,G=0.252671,B=0.135675,A=1.000000)" (LocalVariables|Get%25_ButtonX) (LocalVariables|Get%25_ButtonY) 0 1.0 false)
              (Class|HUD|DrawLine (LocalVariables|Get%25_ButtonX) (LocalVariables|Get%25_ButtonY) (.X (Math|Vector2D|BreakVector2D (LocalVariables|Get%25_ButtonRightBottomPos))) (.Y (Math|Vector2D|BreakVector2D (LocalVariables|Get%25_ButtonRightBottomPos))) "(R=0.118552,G=0.024244,B=1.000000,A=1.000000)")
              (Class|HUD|AddHitBox (LocalVariables|Get%25_ButtonLeftTopPos) (Math|Vector2D|MakeVector2D (LocalVariables|Get%25_ToolsContentItemWidth) (Variables|Tools|GetToolsButtonHeight)) (LocalVariables|Get%25_ID) false))))
        (elif (Utilities|Name|Equal(Name) _selectedtool _id_2)
          (for (_array_element_2 _array_index_2) _segmentlist
            (LocalVariables|Set%25_i _array_index_2)
            (LocalVariables|Set%25_ID (.ID (Utilities|Struct|BreakST_Segment _array_element_2)))
            (LocalVariables|Set%25_title (.Title (Utilities|Struct|BreakST_Segment _array_element_2)))
            (Utilities|FlowControl|Sequence
              (:then_0
                (Utilities|FlowControl|Sequence
                  (:then_0
                    (LocalVariables|Set%25_ButtonXIndex (Math|Integer|%(Integer) (LocalVariables|Get%25_i) _toolscontentitemperline))
                    (LocalVariables|Set%25_ButtonYIndex (/ (LocalVariables|Get%25_i) _toolscontentitemperline))
                    (LocalVariables|Set%25_ButtonX (+ (* (LocalVariables|Get%25_ButtonXIndex) (LocalVariables|Get%25_ToolsContentItemWidth)) (+ _x _toolscontentmargin (* (LocalVariables|Get%25_ButtonXIndex) _toolscontentitemspacing))))
                    (LocalVariables|Set%25_ButtonY (+ (+ (* (LocalVariables|Get%25_ButtonYIndex) _toolsbuttonheight_2) _toolsbuttonheight_2) (+ _y _toolscontentmargin (* (LocalVariables|Get%25_ButtonYIndex) _toolscontentitemspacing))))
                    (LocalVariables|Set%25_ButtonLeftTopPos (Math|Vector2D|MakeVector2D (+ (* (LocalVariables|Get%25_ButtonXIndex) (LocalVariables|Get%25_ToolsContentItemWidth)) (+ _x _toolscontentmargin (* (LocalVariables|Get%25_ButtonXIndex) _toolscontentitemspacing))) (+ (+ (* (LocalVariables|Get%25_ButtonYIndex) _toolsbuttonheight_2) _toolsbuttonheight_2) (+ _y _toolscontentmargin (* (LocalVariables|Get%25_ButtonYIndex) _toolscontentitemspacing)))))
                    (LocalVariables|Set%25_ButtonRightBottomPos (+ (Math|Vector2D|MakeVector2D (+ (* (LocalVariables|Get%25_ButtonXIndex) (LocalVariables|Get%25_ToolsContentItemWidth)) (+ _x _toolscontentmargin (* (LocalVariables|Get%25_ButtonXIndex) _toolscontentitemspacing))) (+ (+ (* (LocalVariables|Get%25_ButtonYIndex) _toolsbuttonheight_2) _toolsbuttonheight_2) (+ _y _toolscontentmargin (* (LocalVariables|Get%25_ButtonYIndex) _toolscontentitemspacing)))) (Math|Vector2D|MakeVector2D (LocalVariables|Get%25_ToolsContentItemWidth) _toolsbuttonheight_2))))))
              (:then_1
                (HUD|DrawRect "(R=0.208383,G=0.540137,B=0.995000,A=1.000000)" (LocalVariables|Get%25_ButtonX) (LocalVariables|Get%25_ButtonY) (LocalVariables|Get%25_ToolsContentItemWidth) (Variables|Tools|GetToolsButtonHeight))
                (HUD|DrawText (LocalVariables|Get%25_title) "(R=0.335000,G=0.252671,B=0.135675,A=1.000000)" (LocalVariables|Get%25_ButtonX) (LocalVariables|Get%25_ButtonY) 0 1.0 false)
                (Class|HUD|DrawLine (LocalVariables|Get%25_ButtonX) (LocalVariables|Get%25_ButtonY) (.X (Math|Vector2D|BreakVector2D (LocalVariables|Get%25_ButtonRightBottomPos))) (.Y (Math|Vector2D|BreakVector2D (LocalVariables|Get%25_ButtonRightBottomPos))) "(R=0.118552,G=0.024244,B=1.000000,A=1.000000)")
                (Class|HUD|AddHitBox (LocalVariables|Get%25_ButtonLeftTopPos) (Math|Vector2D|MakeVector2D (LocalVariables|Get%25_ToolsContentItemWidth) (Variables|Tools|GetToolsButtonHeight)) (LocalVariables|Get%25_ID) false)))))))
    (:then_1
      ;[1 1 1] Debug
      (Debug|DebugThis "_ToolsContentItemWidth" (Utilities|String|ToString(Float) (LocalVariables|Get%25_ToolsContentItemWidth))))))

(fn UpdateValues
  ;[1 1 1] SelectedTool
  (for _array_element (.ToolList (Utilities|Struct|BreakST_Tools (Variables|Tools|GetToolsListStruct)))
    (if true
      (Variables|Global|SetSelectedTool (.ID (Utilities|Struct|BreakST_Tool _array_element))))))